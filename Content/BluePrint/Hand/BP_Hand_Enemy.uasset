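; BP_Hand_Enemy is a hand enemy that advances on its target spawn point, deducting its score there on arrival.
; On BeginPlay it makes a probability-weighted pick from DT_Hand, setting speed, hit count, score and texture on a dynamic material.
; Tick moves it along local X while interpolating rotation toward the target.
; Hits pause movement for a timeline-driven knockback; the lethal hit pushes it away, then destroys it.
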(event Custom|I%20Am%20Deaed
  (Variables|Default|SetMoveGate false)
  (Actor|DestroyActor))

(event Custom|BeHit
  (params (HitLocation :type Vector))
  (bind _returnvalue (Transformation|GetActorLocation))
  (bind _tolocation_spawnpoint (Variables|Default|GetToLocation_SpawnPoint))
  (bind _returnvalue_2 (Transformation|GetActorLocation _tolocation_spawnpoint))
  (bind _returnvalue_3 (- _returnvalue _returnvalue_2))
  (bind _returnvalue_4 (Math|Vector|Normalize _returnvalue_3))
  (bind _returnvalue_5 (* _returnvalue_4 1e+01))
  (if (not (Variables|Default|GetInHit))
    (Variables|Default|SetInHit true)
    (bind _result (Math|Integer|IncrementInt (Variables|Default|GetNow_HitNum))
      (:%20%20
        (Variables|Default|SetMoveGate false)
        (if (>= _result (Variables|Default|GetDeadNum))
          (Variables|Default|SetFlyDiration _returnvalue_5)
          (Timeline|Timeline_2 PlayFromStart
            (:Update
              (Transformation|AddActorWorldOffset _returnvalue_5))
            (:Finished
              (CallFunction|IAmDeaed)
              (Variables|Default|SetInHit false)))
          (else
            (Variables|Default|SetFlyDiration (+ (* (Math|Vector|Normalize (- (Transformation|GetActorLocation) (Transformation|GetActorLocation (Variables|Default|GetToLocation_SpawnPoint)))) (Variables|Default|GetFlySpeed)) (* (Math|Vector|Normalize (- (Transformation|GetActorLocation) HitLocation)) 1.0)))
            (bind _newtrack_0 (Timeline|Timeline_1 PlayFromStart)
              (:Update
                (Transformation|AddActorWorldOffset (* (Variables|Default|GetFlyDiration) _newtrack_0)))
              (:Finished
                (Variables|Default|SetMoveGate true)
                (Variables|Default|SetInHit false)))))))))

(event EventBeginPlay
  (CallFunction|Init))

(event Collision|EventActorBeginOverlap
  (params (OtherActor :type Actor%20Object%20Reference)))

(event EventTick
  (params (DeltaSeconds :type Float%20%28single-precision%29))
  (bind _returnvalue (Transformation|GetActorRotation))
  (bind _returnvalue_2 (Transformation|GetActorLocation))
  (bind _returnvalue_3 (Utilities|Time|GetWorldDeltaSeconds))
  (bind _tolocation_spawnpoint (Variables|Default|GetToLocation_SpawnPoint))
  (bind _returnvalue_4 (Transformation|GetActorLocation _tolocation_spawnpoint))
  (bind _returnvalue_5 (Math|Rotator|FindLookatRotation _returnvalue_2 _returnvalue_4))
  (bind _returnvalue_6 (Math|Interpolation|RInterpTo _returnvalue _returnvalue_5 _returnvalue_3 2.0))
  (if (Variables|Default|GetMoveGate)
    (if (<= (Math|Vector|VectorLength (- _returnvalue_2 _returnvalue_4)) 2e+01)
      ;[1 1 1] GameOver
      (Utilities|FlowControl|DoOnce false
        (:Completed
          (Default|DeScore (Variables|Default|GetToLocation_SpawnPoint) (.Score (Utilities|Struct|BreakST_HandEnemyProperty (Variables|Default|GetMyInfo))))
          (Actor|DestroyActor)))
      (else
        (Transformation|AddActorLocalOffset (Math|Vector|MakeVector (* DeltaSeconds (Variables|Default|GetSpeed)) 0.0 0.0) false false)
        (Transformation|SetActorRotation (Math|Rotator|MakeRotator (.roll _returnvalue_6) 0.0 (.yaw _returnvalue_6)))))))

(fn ConstructionScript
  (bind _returnvalue (Rendering|Material|CreateDynamicMaterialInstance (Variables|Default|GetPlane) 0 "/Game/BluePrint/Hand/M_EnemyHand_Texture.M_EnemyHand_Texture" "None" :!class /Script/Engine.PrimitiveComponent))
  (Variables|Default|SetMat _returnvalue))

(fn Init
  (bind _outrownames (DataTable|GetDataTableRowNames "/Game/BluePrint/Model/DT_Hand.DT_Hand"))
  (for _array_element _outrownames
    (bind _returnvalue (Utilities|GetDataTableRow "/Game/BluePrint/Model/DT_Hand.DT_Hand" _array_element)
      (:then
        (Variables|Prob|SetAllProb (+ (Variables|Prob|GetAllProb) (.Prob (Utilities|Struct|BreakST_HandEnemyProperty _returnvalue)))))))
  (Variables|Prob|SetRandomProb (Math|Random|RandomFloatinRange 0.0 (Variables|Prob|GetAllProb)))
  (bind _array_element_2 (Utilities|Array|ForEachLoopwithBreak _outrownames :!label _label)
    (:LoopBody
      (bind _returnvalue_2 (Utilities|GetDataTableRow "/Game/BluePrint/Model/DT_Hand.DT_Hand" _array_element_2)
        (:then
          (Variables|Prob|SetRandomProb (- (Variables|Prob|GetRandomProb) (.Prob (Utilities|Struct|BreakST_HandEnemyProperty _returnvalue_2))))
          (if (<= (Variables|Prob|GetRandomProb) 0.0)
            (Variables|Default|SetMyInfo _returnvalue_2)
            (goto _label Break)))))
    (:Completed
      (Variables|Default|SetSpeed (.Speed (Utilities|Struct|BreakST_HandEnemyProperty (Variables|Default|GetMyInfo))))
      (Variables|Default|SetDeadNum (.HitNum (Utilities|Struct|BreakST_HandEnemyProperty (Variables|Default|GetMyInfo))))
      (Rendering|Material|SetTextureParameterValue (Variables|Default|GetMat) "Texture" (.Image (Utilities|Struct|BreakST_HandEnemyProperty (Variables|Default|GetMyInfo)))))))