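; BP_PlayerHand is the player's hand actor, which circles a centre point and hits BP_Hand_Enemy actors that overlap its box.
; A game mode event with the Ticket value runs Init, which takes the centre from CurrentActor, creates the circle material and enables input.
; A and D axes adjust a clamped target radius.
; Tick eases toward it, updates the material and moves the hand tangentially with radial correction.
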(event OnComponentBeginOverlap(Box)
  (params (OverlappedComponent :type Primitive%20Component%20Object%20Reference) (OtherActor :type Actor%20Object%20Reference) (OtherComp :type Primitive%20Component%20Object%20Reference) (OtherBodyIndex :type Integer) (bFromSweep :type Boolean) (SweepResult :type Hit%20Result%20Structure%20%28by%20ref%29))
  (bind _asbp_hand_enemy (Utilities|Casting|CastToBP_Hand_Enemy OtherActor))
  (Default|BeHit _asbp_hand_enemy (Transformation|GetActorLocation)))

(event Custom|CustomEvent_0
  (params (NewParam :type EM_GameState%20Enum :default "NewEnumerator0"))
  (switch Utilities|FlowControl|Switch|SwitchonEM_GameState NewParam
    (:NewEnumerator0
      (CallFunction|Init)
      (Development|PrintString "Hello"))))

(event EventBeginPlay
  (bind _asbp_game_mode (Utilities|Casting|CastToBP_GameMode (Game|GetGameMode)))
  (EventDispatchers|BindEventtoEventEEEEEEEEEEBeginPlay _asbp_game_mode (delegate Custom|CustomEvent_0)))

(event EventTick
  (params (DeltaSeconds :type Float%20%28single-precision%29))
  (bind _returnvalue (Transformation|GetActorLocation))
  (bind _centrelocation (Variables|Default|GetCentreLocation))
  (bind _returnvalue_2 (- _centrelocation _returnvalue))
  (bind _returnvalue_3 (Math|Vector|Normalize _returnvalue_2))
  (if (Variables|Default|GetGate)
    (Utilities|FlowControl|Sequence
      (:then_0
        (Variables|Default|SetRange (Math|Interpolation|FInterpTo (Variables|Default|GetRange) (Variables|Default|GetRange_lerp) DeltaSeconds 3.0)))
      (:then_1
        (Rendering|Material|SetScalarParameterValue (Variables|Default|GetPlaneMAT) "Radius" (Variables|Default|GetRange) :!class /Script/Engine.MaterialInstanceDynamic)
        (Transformation|AddActorWorldOffset (+ (* (Math|Vector|CrossProduct _returnvalue_3 "0, 0,1.000000") (* (Variables|Default|GetSpeed) DeltaSeconds)) (* _returnvalue_3 (- (Math|Vector|VectorLength (- (Variables|Default|GetCentreLocation) (Transformation|GetActorLocation))) (Variables|Default|GetRange)))))))))

(event Input|AxisEvents|InputAxisA
  (params (AxisValue :type Float%20%28single-precision%29))
  (Variables|Default|SetRange_lerp (Math|Float|Clamp(Float) (+ (Variables|Default|GetRange_lerp) (* AxisValue (Variables|Default|GetAdd_Unit))) (Variables|Default|GetAdd_Min) (Variables|Default|GetAdd_Max))))

(event Input|AxisEvents|InputAxisD
  (params (AxisValue :type Float%20%28single-precision%29))
  (Variables|Default|SetRange_lerp (Math|Float|Clamp(Float) (+ (Variables|Default|GetRange_lerp) (* (* (Variables|Default|GetAdd_Unit) -1.0) (* (Variables|Default|GetAdd_Unit) AxisValue))) (Variables|Default|GetAdd_Min) (Variables|Default|GetAdd_Max))))

(fn ConstructionScript)

(fn Init
  (bind _currentactor (Variables|Default|GetCurrentActor))
  (Utilities|FlowControl|Sequence
    (:then_0
      (Utilities|IsValid _currentactor
        (:Is%20Valid
          (bind _output_get (Variables|Default|SetCentreLocation (Transformation|GetActorLocation _currentactor)))
          (bind _returnvalue (Rendering|Material|CreateDynamicMaterialInstance (Variables|Default|GetPlane1) 0 "/Game/BluePrint/Hand/M_Circle_Hit_Inst.M_Circle_Hit_Inst" "None" :!class /Script/Engine.PrimitiveComponent))
          (Variables|Default|SetPlaneMAT _returnvalue)
          (Rendering|Material|SetVectorParameterValue _returnvalue "Centre" (Math|Conversions|ToLinearColor(Vector) _output_get) :!class /Script/Engine.MaterialInstanceDynamic))))
    (:then_1
      (CallFunction|BeControl1)
      (Variables|Default|SetGate true))))

(fn BeControl1
  (Input|EnableInput (Game|GetPlayerController 0)))