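; BP_HandSpawnPoint is a spawner that periodically creates BP_Hand_Enemy actors around its own location.
; Tick accumulates time and calls Spawn whenever a gate is reached, then re-rolls the gate within a random min/max range.
; Spawn picks a random point on the edge of an X/Y rectangle centred on the actor.
; Each enemy faces the centre and receives this spawn point as its ToLocationSpawnPoint.
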(event Custom|Spawn
  (bind _returnvalue (Math|Random|RandomBool))
  (bind _x (Variables|Default|GetX))
  (bind _y (Variables|Default|GetY))
  (bind _y_2 (Variables|Default|GetY))
  (bind _x_2 (Variables|Default|GetX))
  (Variables|Default|SetTempSpawnLocation (+ (Transformation|GetActorLocation) (select (Math|Random|RandomBool) (Math|Vector|MakeVector (select _returnvalue (* _x -1.0) _x) (Math|Random|RandomFloatinRange (* _y -1.0) _y) 0.0) (Math|Vector|MakeVector (Math|Random|RandomFloatinRange (* _x_2 -1.0) _x_2) (select _returnvalue (* _y_2 -1.0) _y_2) 0.0))))
  (Game|SpawnActorfromClass "/Game/BluePrint/Hand/BP_Hand_Enemy.BP_Hand_Enemy_C" (Math|Transform|MakeTransform (Variables|Default|GetTempSpawnLocation) (Math|Rotator|FindLookatRotation (Variables|Default|GetTempSpawnLocation) (Transformation|GetActorLocation)) "1,1,1") "Undefined" 0 self 0))

(event EventBeginPlay)

(event EventTick
  (params (DeltaSeconds :type Float%20%28single-precision%29))
  (bind _output_get (Variables|Default|SetCount (+ (Variables|Default|GetCount) DeltaSeconds)))
  (if (>= _output_get (Variables|Default|GetTimeGate))
    (Variables|Default|SetCount 0.0)
    (Variables|Default|SetTimeGate (Math|Random|RandomFloatinRange (Variables|Default|GetradnomTime_Min) (Variables|Default|GetradnomTime_Max)))
    (CallFunction|Spawn)))

(fn ConstructionScript)