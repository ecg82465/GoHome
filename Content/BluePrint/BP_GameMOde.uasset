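; Game mode Blueprint that handles the game-over screen and transitions between the Train and Home stages.
; GameOver creates the U_GameOver widget if none is valid, caches it and adds it to the viewport.
; ToNextLevel switches on the target stage and uses "ce" console commands to trigger the BeginTrain or BeginHome custom events.
; The Home branch also calls EventEEEEEEEEEEBeginPlay with Home.
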(event Custom|GameOver
  (Utilities|IsValid (Variables|Default|GetGameOver_Umg)
    (:Is%20Valid
      _)
    (:Is%20Not%20Valid
      (bind _returnvalue (UserInterface|CreateWidget "/Game/BluePrint/Umg/U_GameOver.U_GameOver_C"))
      (Variables|Default|SetGameOver_Umg _returnvalue)))
  (UserInterface|Viewport|AddtoViewport (Variables|Default|GetGameOver_Umg) 0))

(event Custom|ToNextLevel
  (params (NewParam :type EM_GameState%20Enum :default "NewEnumerator0"))
  (switch Utilities|FlowControl|Switch|SwitchonEM_GameState NewParam
    (:NewEnumerator1
      (Development|ExecuteConsoleCommand "ce BeginTrain" 0))
    (:NewEnumerator3
      (Development|ExecuteConsoleCommand "ce BeginHome" 0)
      (Default|CallEventEEEEEEEEEEBeginPlay "NewEnumerator3"))))

(fn ConstructionScript)