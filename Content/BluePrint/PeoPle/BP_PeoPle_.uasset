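; BP_PeoPle_ is a player-controlled character that walks forward and back and turns left and right.
; On BeginPlay, Init makes the first player controller possess it and sets the character movement's walk speed from MaxSpeed.
; The W_S axis adds movement along the actor's forward vector, while the MoveRight axis adds controller yaw, so sideways input rotates rather than strafes.
; An unconnected debug print of the right-vector rotation remains.
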(event EventBeginPlay
  (CallFunction|Init))

(event Input|AxisEvents|InputAxisW_S
  (params (AxisValue :type Float%20%28single-precision%29))
  (Pawn|Input|AddMovementInput (Transformation|GetActorForwardVector) AxisValue false))

(event Input|AxisEvents|InputAxisMoveRight
  (params (AxisValue :type Float%20%28single-precision%29))
  (Pawn|Input|AddControllerYawInput AxisValue))

(fn ConstructionScript)

(fn Init
  (Pawn|Possess (Game|GetPlayerController 0) self)
  (Variables|/Script/Engine.CharacterMovementComponent|SetMaxWalkSpeed (Variables|Character|GetCharacterMovement) (Variables|Default|GetMaxSpeed)))