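; Player character (likely for a train level) that self-possesses, walks along its forward axis and turns with yaw input through a crowd of BP_PeoPle.
; A SaySomeThing overlap tracks nearby people without duplicates.
; Every three seconds it calls Pacify on those whose projection onto the BP_EndWall arrow is at or below its own.
; BePush applies a horizontal impulse; the IsInPush-setting and timeline-retreat branches are unreachable.
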(event OnComponentBeginOverlap(SaySomeThing)
  (params (OverlappedComponent :type Primitive%20Component%20Object%20Reference) (OtherActor :type Actor%20Object%20Reference) (OtherComp :type Primitive%20Component%20Object%20Reference) (OtherBodyIndex :type Integer) (bFromSweep :type Boolean) (SweepResult :type Hit%20Result%20Structure%20%28by%20ref%29))
  ;[1 1 1] Check PeoPle
  (bind _asbp_peo_ple (Utilities|Casting|CastToBP_PeoPle OtherActor))
  (bind _go (CallFunction|CheckList _asbp_peo_ple))
  (if _go
    (Utilities|Array|Add (Variables|Default|GetAroundList) _asbp_peo_ple)))

(event OnComponentEndOverlap(SaySomeThing)
  (params (OverlappedComponent :type Primitive%20Component%20Object%20Reference) (OtherActor :type Actor%20Object%20Reference) (OtherComp :type Primitive%20Component%20Object%20Reference) (OtherBodyIndex :type Integer))
  ;[1 1 1] Check PeoPle
  (bind _asbp_peo_ple (Utilities|Casting|CastToBP_PeoPle OtherActor))
  (Utilities|Array|RemoveItem (Variables|Default|GetAroundList) _asbp_peo_ple))

(event Custom|BePush
  (params (Location :type Vector) (Normal :type Vector))
  (bind _returnvalue (* Normal -5e+04))
  (bind (_x _y) (Math|Vector|BreakVector _returnvalue))
  ;[1 1 1] BePush
  (Physics|AddImpulse (Variables|Character|GetCharacterMovement) (Math|Vector|MakeVector _x _y 0.0) false)
  (Development|PrintString "Hello")
  (Utilities|FlowControl|Delay 1.0)
  (Variables|Default|SetIsInPush false))

(event EventBeginPlay
  (CallFunction|Init))

(event EventTick
  (params (DeltaSeconds :type Float%20%28single-precision%29))
  (bind _output_get (Variables|Default|SetCD (+ DeltaSeconds (Variables|Default|GetCD))))
  (if (>= _output_get 3.0)
    (Variables|Default|SetCD 0.0)
    (CallFunction|ExcuseMe)))

(event Input|AxisEvents|InputAxisW_S
  (params (AxisValue :type Float%20%28single-precision%29))
  (if (not (Variables|Default|GetIsInPush))
    (Pawn|Input|AddMovementInput (Transformation|GetActorForwardVector) AxisValue false)))

(event Input|AxisEvents|InputAxisMoveRight
  (params (AxisValue :type Float%20%28single-precision%29))
  (Pawn|Input|AddControllerYawInput AxisValue))

(fn ConstructionScript
  (bind _outactors (Actor|GetAllActorsOfClass "/Game/BluePrint/PeoPle/BP_EndWall.BP_EndWall_C"))
  (Variables|Default|SetBP_EndWall (Utilities|Array|Get(acopy) _outactors)))

(fn Init
  (Pawn|Possess (Game|GetPlayerController 0) self)
  (Variables|/Script/Engine.CharacterMovementComponent|SetMaxWalkSpeed (Variables|Character|GetCharacterMovement) (Variables|Default|GetMaxSpeed)))

(fn CheckList
  (params (B :type Object%20Object%20Reference))
  (for _array_element (Variables|Default|GetAroundList)
    (if (== _array_element B)
      (return false)))
  (return true))

(fn ExcuseMe
  (for _array_element (Variables|Default|GetAroundList)
    (if (<= (CallFunction|GetLengthtoWall _array_element) (CallFunction|GetLengthtoWall self))
      (Default|Pacify _array_element self))))

(fn GetLengthtoWall
  (params (NewParam :type Actor%20Object%20Reference))
  (bind _bp_endwall (Variables|Default|GetBP_EndWall))
  (return (Math|Vector|DotProduct (- (Transformation|GetActorLocation NewParam) (Transformation|GetActorLocation _bp_endwall)) (Variables|/Game/BluePrint/PeoPle/BP_EndWall.BP_EndWall_C|GetArrow_Forwad _bp_endwall))))