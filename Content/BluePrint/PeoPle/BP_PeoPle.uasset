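; Crowd NPC character that gets angrier when the player bumps it and shoves the player once anger maxes out.
; The construction script pulls type-specific stats, scale and texture from DE_PeoPle.
; Hits add anger, shown on a TextRender, and at the limit a line trace delivers the push.
; Pacify lowers anger and triggers a timed, Tick-driven sidestep away from the player along the EndWall's axis, then a walk back to spawn.
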(event Custom|Pacify
  (params (Player :type BP%20Player%20Pawn%20Trian%20Object%20Reference))
  ;[1 1 1] Pacify
  (Variables|Default|SetAngerValue (Math|Float|Clamp(Float) (- (Variables|Default|GetAngerValue) 3.0) 0.0 (Variables|Default|GetAngerValue_Max)))
  (Variables|Default|SetMoveGate true)
  (Variables|Default|SetWalkTime 1.2)
  (switch Utilities|FlowControl|Switch|SwitchonEM_PeoPleState (Variables|Default|GetPeoPle_State)
    (:NewEnumerator1
      (CallFunction|ChangeState "NewEnumerator0"))))

(event Custom|PushPlayer)

(event EventBeginPlay
  (CallFunction|Init))

(event Collision|EventHit
  (params (MyComp :type Primitive%20Component%20Object%20Reference) (Other :type Actor%20Object%20Reference) (OtherComp :type Primitive%20Component%20Object%20Reference) (bSelfMoved :type Boolean) (HitLocation :type Vector :default "0, 0, 0") (HitNormal :type Vector :default "0, 0, 0") (NormalImpulse :type Vector :default "0, 0, 0") (Hit :type Hit%20Result%20Structure%20%28by%20ref%29))
  (bind _returnvalue (Transformation|GetActorLocation))
  ;[1 1 1] Push
  (bind _asbp_player_pawn_trian (Utilities|Casting|CastToBP_PlayerPawnTrian Other))
  (Variables|Default|SetPlayer _asbp_player_pawn_trian)
  (Utilities|FlowControl|Delay 0.2)
  (Pawn|Input|AddMovementInput HitNormal 1.0 false)
  (bind _output_get (Variables|Default|SetAngerValue (+ (Variables|Default|GetAngerValue) (Variables|Default|GetAnger_Add))))
  (if (>= _output_get (Variables|Default|GetAngerValue_Max))
    (Utilities|IsValid (Variables|Default|GetPlayer)
      (:Is%20Valid
        (bind _outhit (Collision|LineTraceByChannel _returnvalue (+ (* (- (Transformation|GetActorLocation (Variables|Default|GetPlayer)) _returnvalue) 333.0) _returnvalue) "TraceTypeQuery2" false 0 "ForDuration"))
        (if (.bBlockingHit (Collision|BreakHitResult _outhit))
          (bind _asbp_player_pawn_trian_2 (Utilities|Casting|CastToBP_PlayerPawnTrian (.HitActor (Collision|BreakHitResult _outhit))))
          (Default|BePush _asbp_player_pawn_trian_2 (.Location (Collision|BreakHitResult _outhit)) (.Normal (Collision|BreakHitResult _outhit)) 5e+04))))))

(event EventTick
  (params (DeltaSeconds :type Float%20%28single-precision%29))
  (Utilities|FlowControl|Sequence
    (:then_0
      (Rendering|Components|TextRender|SetText (Variables|Default|GetTextRender) (Utilities|Text|ToText(String) (Utilities|String|Append "Anger:" (Utilities|String|ToString(Float) (Variables|Default|GetAngerValue))))))
    (:then_1
      (if (Variables|Default|GetMoveGate)
        (switch Utilities|FlowControl|Switch|SwitchonEM_PeoPleState (Variables|Default|GetPeoPle_State)
          (:NewEnumerator0
            (CallFunction|Retreat))
          (:NewEnumerator1
            (CallFunction|GiveBack)))))))

(fn ConstructionScript
  (bind _outrownames (DataTable|GetDataTableRowNames "/Game/BluePrint/Model/DE_PeoPle.DE_PeoPle"))
  (bind _array_element (Utilities|Array|ForEachLoopwithBreak _outrownames :!label _label)
    (:LoopBody
      (bind _returnvalue (Utilities|GetDataTableRow "/Game/BluePrint/Model/DE_PeoPle.DE_PeoPle" _array_element)
        (:then
          (if (Utilities|Enum|Equal(Enum) (.Type (Utilities|Struct|BreakST_PeoPleProperty _returnvalue)) (Variables|Default|GetEM_People))
            (Variables|Default|SetMyInfo _returnvalue)
            (goto _label Break)))))
    (:Completed
      (Transformation|SetActorScale3D (Math|Vector|MakeVector (.Scale (Utilities|Struct|BreakST_PeoPleProperty (Variables|Default|GetMyInfo))) (.Scale (Utilities|Struct|BreakST_PeoPleProperty (Variables|Default|GetMyInfo))) 1.0))
      (bind _returnvalue_2 (Rendering|Material|CreateDynamicMaterialInstance (Variables|Default|GetPlane) 0 "/Game/BluePrint/Hand/M_EnemyHand_Texture.M_EnemyHand_Texture" "None" :!class /Script/Engine.PrimitiveComponent))
      (Rendering|Material|SetTextureParameterValue _returnvalue_2 "Texture" (.Texture (Utilities|Struct|BreakST_PeoPleProperty (Variables|Default|GetMyInfo)))))))

(fn Init
  (params (Player :type BP%20Player%20Pawn%20Trian%20Object%20Reference))
  (bind _myinfo (Variables|Default|GetMyInfo))
  (Utilities|FlowControl|Sequence
    (:then_0
      (bind _outactors (Actor|GetAllActorsOfClass "/Game/BluePrint/PeoPle/BP_PlayerPawnTrian.BP_PlayerPawnTrian_C"))
      (Variables|Default|SetPlayer (Utilities|Array|Get(acopy) _outactors))
      (bind _outactors_2 (Actor|GetAllActorsOfClass "/Game/BluePrint/PeoPle/BP_EndWall.BP_EndWall_C"))
      (Variables|Default|SetEndWall (Utilities|Array|Get(acopy) _outactors_2))
      (Variables|Default|SetSpawnLocation (Transformation|GetActorLocation)))
    (:then_1
      (Variables|Default|SetMaxSpeed (.maxspeed _myinfo))
      (Variables|Default|SetAngerValue_Max (.maxanger _myinfo))
      (Variables|Default|SetAnger_Add (.angeraddspeed _myinfo))
      (Variables|/Script/Engine.CharacterMovementComponent|SetMaxWalkSpeed (Variables|Character|GetCharacterMovement) (Variables|Default|GetMaxSpeed)))))

(fn Retreat
  (bind _returnvalue (Transformation|GetActorLocation))
  (bind _endwall (Variables|Default|GetEndWall))
  (bind _player (Variables|Default|GetPlayer))
  (bind _returnvalue_2 (Transformation|GetActorLocation _player))
  (bind _arrow_right (Variables|/Game/BluePrint/PeoPle/BP_EndWall.BP_EndWall_C|GetArrow_Right _endwall))
  (bind _returnvalue_3 (- _returnvalue _returnvalue_2))
  (bind _returnvalue_4 (Math|Vector|Normalize _returnvalue_3))
  (Variables|Default|SetWalkTime (- (Variables|Default|GetWalkTime) (Utilities|Time|GetWorldDeltaSeconds)))
  (if (<= (Variables|Default|GetWalkTime) 0.0)
    (CallFunction|ChangeState "NewEnumerator1")
    (else
      (Pawn|Input|AddMovementInput (+ (* _returnvalue_4 0.3) (* _arrow_right (select (<= (Math|Vector|DotProduct _returnvalue_4 _arrow_right) 0.0) (Math|Float|MakeLiteralFloat -1.0) (Math|Float|MakeLiteralFloat 1.0)))) 1.0 false))))

(fn GiveBack
  (bind _returnvalue (Transformation|GetActorLocation))
  (bind _spawnlocation (Variables|Default|GetSpawnLocation))
  (bind _returnvalue_2 (- _spawnlocation _returnvalue))
  (if (<= (Math|Vector|VectorLength _returnvalue_2) 1e+01)
    (Variables|Default|SetMoveGate false)
    (else
      (Pawn|Input|AddMovementInput _returnvalue_2 1.0 false))))

(fn ChangeState
  (params (PeoPle_State :type EM_PeoPleState%20Enum :default "NewEnumerator0"))
  (Variables|Default|SetPeoPle_State PeoPle_State))