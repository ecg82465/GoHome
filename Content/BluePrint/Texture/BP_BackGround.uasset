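; BP_BackGround is a background actor that shows a selectable texture from an array on a plane.
; The construction script creates a dynamic M_Texture material instance and sets its Texture parameter to the TextureArray entry at index Num.
; Tick reapplies that texture every frame, and a RepNotify function performs the same update on replication.
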(event EventBeginPlay)

(event Collision|EventActorBeginOverlap
  (params (OtherActor :type Actor%20Object%20Reference)))

(event EventTick
  (params (DeltaSeconds :type Float%20%28single-precision%29))
  (Rendering|Material|SetTextureParameterValue (Variables|Default|GetMat) "Texture" (Utilities|Array|Get(acopy) (Variables|Default|GetTextureArray) (Variables|Default|GetNum))))

(fn ConstructionScript
  (bind _returnvalue (Rendering|Material|CreateDynamicMaterialInstance (Variables|Default|GetPlane) 0 "/Game/Mateirals/M_Texture.M_Texture" "None" :!class /Script/Engine.PrimitiveComponent))
  (Variables|Default|SetMat _returnvalue)
  (Rendering|Material|SetTextureParameterValue (Variables|Default|GetMat) "Texture" (Utilities|Array|Get(acopy) (Variables|Default|GetTextureArray) (Variables|Default|GetNum))))

(fn OnRepNewVar0
  (Rendering|Material|SetTextureParameterValue (Variables|Default|GetMat) "Texture" (Utilities|Array|Get(acopy) (Variables|Default|GetTextureArray) (Variables|Default|GetNum))))