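; Player controller that shows the mouse cursor and tracks what lies under it in the world.
; Every tick it deprojects the mouse position, runs a Visibility line trace along that ray and stores the result in HitLocation.
; Left mouse press and release toggle a TraceGate flag, but the branch that reads it is disconnected, so tracing runs regardless of the button.
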(event EventBeginPlay
  (Variables|Default|SetbShowMouseCursor true))

(event EventTick
  (params (DeltaSeconds :type Float%20%28single-precision%29))
  (bind (_worldlocation _worlddirection) (Game|Player|ConvertMouseLocationToWorldSpace))
  (bind _outhit (Collision|LineTraceByChannel _worldlocation (+ _worldlocation (* _worlddirection 6e+03)) "TraceTypeQuery1" false 0 "None"))
  (Variables|Default|SethitLocation _outhit))

(event Input|MouseEvents|LeftMouseButton
  (params (Key :type Key%20Structure))
  (:Pressed
    (Variables|Default|SetTraceGate true))
  (:Released
    (Variables|Default|SetTraceGate false)))

(fn ConstructionScript)